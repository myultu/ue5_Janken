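; Game mode for a hand-selection battle game, managing which players are battlers by their join-order ID.
; PostLogin binds to JanGamestate's winner event, assigns IDs and battler status, and refreshes battler standby while players don't exceed the battler count.
; Logout shifts higher IDs down, promoting waiting players.
; Winner determination is a stub: it prints, reports a fixed 0, then lets player controllers select again.
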(event Custom|E-determiningTheWinner
  (params (SelectedHands :type Array%20of%20Integers))
  (Development|PrintString "判定ですぞ")
  (Default|E-finishedDetermining (Variables|Default|GetGS-jan))
  (CallFunction|AllowBattlerstoSelect))

(event EventPostLogin
  (params (NewPlayer :type Player%20Controller%20Object%20Reference))
  (Utilities|FlowControl|Sequence
    (:then_0
      (Utilities|FlowControl|DoOnce false
        (:Completed
          (bind _asjan_gamestate (Utilities|Casting|CastToJanGamestate (Game|GetGameState))
            (:then
              (bind _output_get (Variables|Default|SetGS-jan _asjan_gamestate))
              (EventDispatchers|BindEventtoEd-determiningtheWinner _output_get (EventDispatchers|CreateEvent :!event Custom|E-determiningTheWinner)))
            (:CastFailed
              (Utilities|String|LogString "castToJanGamestate failed. @JanGamemode:BeginPlay"))))))
    (:then_1
      (bind (_newpc_jan _newps_jan) (CallFunction|GetNewPlayerControllerandState NewPlayer))
      (if (and (Utilities|IsValid _newpc_jan) (Utilities|IsValid _newps_jan))
        (CallFunction|VoidNewPlayerEvents _newpc_jan _newps_jan)
        (CallFunction|VoidBattlersonStandby)))))

(event EventOnLogout
  (params (ExitingController :type Controller%20Object%20Reference))
  (bind _asjan_playerstate (Utilities|Casting|CastToJanPlayerstate (Variables|/Script/Engine.Controller|GetPlayerState ExitingController))
    (:then
      (Utilities|String|LogString (Utilities|String|Append "ID:" (Utilities|String|ToString(Integer) (Default|GetPlayerIDNum _asjan_playerstate)) " player exited."))
      (for _index (range 0 (Utilities|Array|LastIndex (Variables|/Script/Engine.GameStateBase|GetPlayerArray (Variables|Default|GetGS-jan))))
        (bind (_ps_applicable _newpid) (CallFunction|FindStatestoRewritePID (Default|GetPlayerIDNum _asjan_playerstate) _index))
        (Utilities|IsValid _ps_applicable
          (:Is%20Valid
            (bind _isbattler (CallFunction|IsSmallerThanBNUM _newpid))
            (Default|E-updatePlayerID _ps_applicable _newpid _isbattler))))
      (CallFunction|VoidBattlersonStandby))
    (:CastFailed
      (Utilities|String|LogString "castToJanPlayerstate failed."))))

(fn ConstructionScript)

(fn GetNewPlayerControllerandState
  (params (NewPC :type Player%20Controller%20Object%20Reference))
  (Utilities|FlowControl|Sequence
    (:then_0
      (bind _asjan_playercontroller (Utilities|Casting|CastToJanPlayercontroller NewPC)
        (:then
          (bind _asjan_playerstate (Utilities|Casting|CastToJanPlayerstate (Variables|/Script/Engine.Controller|GetPlayerState NewPC))
            (:then
              (Utilities|String|LogString "New Player joined!")
              (return _asjan_playercontroller _asjan_playerstate))
            (:CastFailed
              (Utilities|String|LogString "castToJanPlayerstate  failed. @JanGamemode:GetNewPlayerControllerAndState"))))
        (:CastFailed
          (Utilities|String|LogString "castToJanPlayercontroller  failed. @JanGamemode:GetNewPlayerControllerAndState"))))
    (:then_1
      (return 0 0))))

(fn IsSmallerThanBNUM
  (params (PID :type Integer))
  (bind _returnvalue (Game|GetGameState))
  (Utilities|IsValid _returnvalue
    (:Is%20Valid
      (bind _asjan_gamestate (Utilities|Casting|CastToJanGamestate _returnvalue)
        (:then
          (return (> (Default|GetBATTLERSNUM _asjan_gamestate) PID)))
        (:CastFailed
          (Utilities|String|LogString "castToJanGamestate  failed. @JanPlayerstate:IsSmallerThanB_NUM")
          (return false))))))

(fn VoidNewPlayerEvents
  (params (newPC-jan :type Jan%20Playercontroller%20Object%20Reference) (newPS-jan :type Jan%20Playerstate%20Object%20Reference))
  (bind _returnvalue (Class|GameplayStatics|GetNumPlayerStates))
  (bind _returnvalue_2 (- _returnvalue 1))
  (Default|E-joinNewPlayer newPC-jan)
  (bind _isbattler (CallFunction|IsSmallerThanBNUM _returnvalue_2))
  (Default|E-joinNewPlayer newPS-jan _returnvalue_2 _isbattler)
  (Default|E-joinNewPlayer (Variables|Default|GetGS-jan) newPC-jan)
  (return))

(fn VoidBattlersonStandby
  (if (>= (Default|GetBATTLERSNUM (Variables|Default|GetGS-jan)) (Class|GameplayStatics|GetNumPlayerStates))
    (bind _index (Utilities|FlowControl|ForLoopwithBreak 0 (- (Class|GameplayStatics|GetNumPlayerStates) 1) :!label _label)
      (:LoopBody
        (bind _isbattler (CallFunction|IsSmallerThanBNUM _index))
        (if _isbattler
          (for _array_element (Variables|/Script/Engine.GameStateBase|GetPlayerArray (Variables|Default|GetGS-jan))
            (bind _asjan_playerstate (Utilities|Casting|CastToJanPlayerstate _array_element)
              (:then
                (bind _output_get (LocalVariables|SetpossibilityTargetAsPS-jan _asjan_playerstate))
                (if (== (Default|GetPlayerIDNum _output_get) _index)
                  (Utilities|IsValid (Game|GetPlayerController (LocalVariables|GetpossibilityTargetAsPS-jan))
                    (:Is%20Valid
                      (bind _asjan_playercontroller (Utilities|Casting|CastToJanPlayercontroller (Game|GetPlayerController (LocalVariables|GetpossibilityTargetAsPS-jan)))
                        (:then
                          (bind _output_get_2 (LocalVariables|SettargetPC-jan _asjan_playercontroller))
                          (Default|E-standby _output_get_2 (> (Default|GetBATTLERSNUM (Variables|Default|GetGS-jan)) (Class|GameplayStatics|GetNumPlayerStates))))
                        (:CastFailed
                          (Utilities|String|LogString "castToJanPlayercontroller  failed. @JanGamemode:voidBattlersOnStandby"))))
                    (:Is%20Not%20Valid
                      (Utilities|String|LogString "IsNotValid: GetPlayerController @JanGamemode:voidBattlersOnStandby")))))
              (:CastFailed
                (Utilities|String|LogString "castToJanPlayerstate failed. @JanGamemode:voidBattlersOnStandby"))))
          (else
            (goto _label Break))))
      (:Completed
        (return)))
    (else
      (return))))

(fn FindStatestoRewritePID
  (params (basePID :type Integer) (index :type Integer))
  (bind _asjan_playerstate (Utilities|Casting|CastToJanPlayerstate (Utilities|Array|Get(acopy) (Variables|/Script/Engine.GameStateBase|GetPlayerArray (Variables|Default|GetGS-jan)) index))
    (:then
      (bind _output_get (LocalVariables|Setps _asjan_playerstate))
      (LocalVariables|Setpid (Default|GetPlayerIDNum _output_get))
      (if (> (LocalVariables|Getpid) basePID)
        (return (LocalVariables|Getps) (- (LocalVariables|Getpid) 1))
        (else
          (return 0 (LocalVariables|Getpid)))))
    (:CastFailed
      (Utilities|String|LogString "castToJanPlayerstate  failed. @JanGamestate:findStatesToRewritePID")
      (return 0 0))))

(fn AllowBattlerstoSelect
  (for _index (range 0 (Utilities|Array|LastIndex (Variables|/Script/Engine.GameStateBase|GetPlayerArray (Variables|Default|GetGS-jan))))
    (Utilities|IsValid (Game|GetPlayerController (Game|GetPlayerState _index))
      (:Is%20Valid
        (bind _asjan_playercontroller (Utilities|Casting|CastToJanPlayercontroller (Game|GetPlayerController (Game|GetPlayerState _index)))
          (:then
            (Default|E-finishedDetermining _asjan_playercontroller))
          (:CastFailed
            (Utilities|String|LogString "castToJanPlayercontroller  failed. @JanGamemode:allowBattlersToSelect"))))
      (:Is%20Not%20Valid
        (Utilities|String|LogString "IsNotValid: GetPlayerController @JanGamemode:allowBattlersToSelect"))))
  (return))