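; Player controller for a multiplayer rock-paper-scissors (janken) game that bridges each player's UI and the match logic.
; On join it creates the Uijanken widget, labeled host or client by authority, and binds its hand-click event.
; A first pick is stored on the JanPlayerstate, then broadcast with controller and player ID through an event dispatcher.
; Standby and selection-phase events toggle waiting text and input lock; the back button opens Home.
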(event Ed-ClickedBack(UI-jan)
  (Game|OpenLevel(byObjectReference) "/Game/home.home"))

(event Custom|E-standby
  (params (isWaitingBattlers :type Boolean))
  (bind _ui_jan (Variables|Default|GetUI-jan))
  (Utilities|IsValid _ui_jan
    (:Is%20Valid
      (Default|E-showWaitingTxt _ui_jan isWaitingBattlers)
      (Default|E-preventSelectingBjan _ui_jan isWaitingBattlers))
    (:Is%20Not%20Valid
      (Utilities|String|LogString "IsNotValid: GetUi-janken @JanPlayercontroller:E-standby"))))

(event Custom|E-joinNewPlayer
  (Networking|SwitchHasAuthority
    (:Authority
      (Variables|Default|SetroleName "ホスト"))
    (:Remote
      (Variables|Default|SetroleName "クライアント")))
  (bind _returnvalue (UserInterface|CreateWidget "/Game/UIHUD/ui-janken.ui-janken_C" self (Variables|Default|GetroleName)))
  (bind _output_get (Variables|Default|SetUI-jan _returnvalue))
  (UserInterface|Viewport|AddtoViewport _output_get 0)
  (EventDispatchers|BindEventtoEd-ClickedGu _output_get (EventDispatchers|CreateEvent :!event Custom|E-clickedGu)))

(event Custom|E-finishedSelecting
  (Default|E-preventSelectingBjan (Variables|Default|GetUI-jan) true))

(event Custom|E-finishedDetermining
  (Default|E-preventSelectingBjan (Variables|Default|GetUI-jan) false))

(event Custom|E-clickedGu
  (params (hand :type Integer))
  (bind _ps_self (CallFunction|GetReferenceOwnPS-jan))
  (if (not (Default|GetAlreadySelected _ps_self))
    (Default|E-receiveSelectedHand _ps_self hand)
    (CallFunction|E-sendHand self (Default|GetPlayerIDNum _ps_self) (Default|GetSelectedHand _ps_self))))

(event Custom|E-sendHand
  (params (PC-applicable :type Jan%20Playercontroller%20Object%20Reference) (playerIDNum :type Integer) (selectedHand :type Integer))
  (Default|CallEd-sendHand PC-applicable playerIDNum selectedHand))

(fn ConstructionScript)

(fn GetUi-jan
  (return (Variables|Default|GetUI-jan)))

(fn GetReferenceOwnPS-jan
  (bind _playerstate (Variables|GetPlayerState))
  (Utilities|IsValid _playerstate
    (:Is%20Valid
      (bind _asjan_playerstate (Utilities|Casting|CastToJanPlayerstate _playerstate)
        (:then
          (return _asjan_playerstate))
        (:CastFailed
          (Utilities|String|LogString "castToJanPlayerstate  failed. @JanPlayercontroller:getReferenceOwnPS-jan"))))
    (:Is%20Not%20Valid
      (Utilities|String|LogString "IsNotValid: GetPlayerState @JanPlayercontroller:getReferenceOwnPS-jan")))
  (return 0))

(fn GetReferenceGS-jan
  (bind _returnvalue (Game|GetGameState))
  (bind _asjan_gamestate (Utilities|Casting|CastToJanGamestate _returnvalue)
    (:then
      (return _asjan_gamestate))
    (:CastFailed
      (Utilities|String|LogString "castToJanGamestate failed. @JanPlayercontroller:getReferenceGS-jan")
      (Utilities|String|LogString (Utilities|String|Append "これが 
" (Utilities|String|ToString(Object) _returnvalue)))
      (return 0))))