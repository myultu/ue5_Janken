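; Game state for a multiplayer hand-picking match (likely janken) that collects each player's hand and tracks the round result.
; It binds each joining player controller's send-hand dispatcher, storing hands and selected flags by player ID.
; When the flags match an all-true reference array sized to the battler count, it broadcasts the hands for winner determination.
; The finish event records the winner and previous hands, then resets both arrays.
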(event Custom|E-joinNewPlayer
  (params (newPC-jan :type Jan%20Playercontroller%20Object%20Reference))
  (EventDispatchers|BindEventtoEd-sendHand newPC-jan (delegate Custom|E-sendHand))
  (Utilities|String|LogString (Utilities|String|Append "現在この部屋に" (Utilities|String|ToString(Integer) (Class|GameplayStatics|GetNumPlayerStates)) "人います")))

(event Custom|E-sendHand
  (params (PC-applicable :type Jan%20Playercontroller%20Object%20Reference) (playerIDNum :type Integer) (selectedHand :type Integer))
  (Utilities|Array|SetArrayElem (Variables|Default|GethandsSelected) playerIDNum selectedHand)
  (Utilities|Array|SetArrayElem (Variables|Default|GetalreadySelected) playerIDNum true)
  (Default|E-finishedSelecting PC-applicable)
  (if (Utilities|Array|Identical (Variables|Default|GetalreadySelected) (Variables|Default|GetFOR_CHECK_SELECTEDSelected))
    (CallFunction|E-determining)))

(event Custom|E-determining
  (Default|CallEd-determiningtheWinner (Variables|Default|GethandsSelected)))

(event Custom|E-finishedDetermining
  (params (winner :type Integer))
  (Variables|Default|Setwinner winner)
  (Variables|Default|SetbeforeHands (Variables|Default|GethandsSelected))
  (CallFunction|VoidResetArrays))

(fn ConstructionScript
  (bind _battlers_num (Variables|Default|GetBATTLERS_NUM))
  ;[1 1 1] 配列の初期化
  (Utilities|Array|Resize (Variables|Default|GethandsSelected) _battlers_num)
  (Utilities|Array|Resize (Variables|Default|GetalreadySelected) _battlers_num)
  (for _index (range 0 (- _battlers_num 1))
    (Utilities|Array|Add (Variables|Default|GetFOR_CHECK_SELECTEDSelected) true))
  (CallFunction|VoidResetArrays))

(fn GetBATTLERSNUM
  (return (Variables|Default|GetBATTLERS_NUM)))

(fn VoidResetArrays
  (bind _alreadyselected (Variables|Default|GetalreadySelected))
  (bind _handsselected (Variables|Default|GethandsSelected))
  (for _index (range 0 (Utilities|Array|LastIndex _handsselected))
    (Utilities|Array|SetArrayElem _handsselected _index -1))
  (for _index_2 (range 0 (Utilities|Array|LastIndex _alreadyselected))
    (Utilities|Array|SetArrayElem _alreadyselected _index_2 false))
  (return))