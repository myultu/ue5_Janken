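; JanPlayerstate is the player state for a hand-selection battle game, holding a player's ID, battler flag and selected hand.
; On join it caches the UI from its owning JanPlayercontroller, stores the ID and role, then updates that UI.
; Events record the chosen hand and reset it once determination finishes.
; Getters expose this state, and a helper compares an ID against the game state's battler count.
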(event Custom|E-joinNewPlayer
  (params (newPID :type Integer) (isBattler :type Boolean))
  (bind _ui_jan (CallFunction|GetReferenceUi-jan))
  (Variables|Default|SetUi-jan _ui_jan)
  (CallFunction|E-updatePlayerID newPID isBattler))

(event Custom|E-updatePlayerID
  (params (NewPID :type Integer) (IsBattler :type Boolean))
  (Variables|Default|SetplayerIDNum NewPID)
  (Variables|Default|SetIs%20Battler IsBattler)
  (CallFunction|E-updateUi))

(event Custom|E-finishedDetermining
  (Variables|Default|SetselectedHand -1)
  (Variables|Default|SetalreadySelected false))

(event Custom|E-receiveSelectedHand
  (params (SelectedHand :type Integer))
  (Variables|Default|SetalreadySelected true)
  (Variables|Default|SetselectedHand SelectedHand))

(event Custom|E-updateUi
  (Default|E-addBjanbyId (Variables|Default|GetUi-jan) (Variables|Default|GetIs%20Battler))
  (Default|E-showId (Variables|Default|GetUi-jan) (Variables|Default|GetplayerIDNum)))

(fn ConstructionScript)

(fn GetPlayerIDNum
  (return (Variables|Default|GetplayerIDNum)))

(fn GetSelectedHand
  (return (Variables|Default|GetselectedHand)))

(fn GetAlreadySelected
  (return (Variables|Default|GetalreadySelected)))

(fn IsSmallerThanBNUM
  (params (PIDNum :type Integer))
  (bind _returnvalue (Game|GetGameState))
  (Utilities|IsValid _returnvalue
    (:Is%20Valid
      (bind _asjan_gamestate (Utilities|Casting|CastToJanGamestate _returnvalue)
        (:then
          (return (> (Default|GetBATTLERSNUM _asjan_gamestate) PIDNum)))
        (:CastFailed
          (Utilities|String|LogString "castToJanGamestate  failed. @JanPlayerstate:IsSmallerThanB_NUM")
          (return false))))))

(fn GetReferencePC-jan
  (bind _asjan_playercontroller (Utilities|Casting|CastToJanPlayercontroller (Components|GetOwner))
    (:then
      (return _asjan_playercontroller))
    (:CastFailed
      (Utilities|String|LogString "castToJanPlayercontroller failed. @JanPlayerstate:getReferencePC-jan")
      (return 0))))

(fn GetReferenceUi-jan
  (bind _pc_jan (CallFunction|GetReferencePC-jan))
  (Utilities|IsValid (Default|GetUi-jan _pc_jan)
    (:Is%20Valid
      (return (Default|GetUi-jan _pc_jan)))
    (:Is%20Not%20Valid
      (Utilities|String|LogString "IsNotValid: getUi-jan @JanPlayerstate:getReferenceUi-jan")
      (return 0))))